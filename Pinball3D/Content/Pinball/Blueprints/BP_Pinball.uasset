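; Playable pinball table actor that takes over the player's camera, locks movement and shows the WD_Pinball widget while in use.
; Custom events drive a charged ball launch and timeline-animated flippers, with Box1 overlaps toggling launch permission.
; Bumper hits delegate to BumperComponent, and the drain hole respawns the ball.
; Shakes tilt the table and restart a timer that locks the flippers after too many shakes, with no unlock here.
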(event `self.ReceiveBeginPlay`
  (`self.CriarNovaBola`)
  (bind _output_get (set `self.RotInicial R` (`SceneComponent.RelativeRotation` (`self.FlipperR`))))
  (set `self.NewRot R` (`KismetMathLibrary.MakeRotator` (.roll _output_get) (.pitch _output_get) (+ (.yaw _output_get) 40.0)))
  (bind _output_get_2 (set `self.RotInicial L` (`SceneComponent.RelativeRotation` (`self.FlipperL`))))
  (set `self.NewRot L` (`KismetMathLibrary.MakeRotator` (.roll _output_get_2) (.pitch _output_get_2) (- (.yaw _output_get_2) 40.0))))

(event `PinballCamera`
  (bind _returnvalue (`GameplayStatics.GetPlayerController` 0))
  ;[0.5457 1 0.4852] Ativa Câmera Pinball
  (`PlayerController.SetViewTargetWithBlend` _returnvalue self 1.0 "VTBlend_Linear" 0.0 false)
  (`Controller.SetIgnoreMoveInput` _returnvalue true)
  (`Controller.SetIgnoreLookInput` _returnvalue true)
  ;[0.5457 1 0.4852] Ativa Interface Pinball
  (bind _returnvalue_2 (`|CreateWidget` "/Game/Pinball/Interface/WD_Pinball.WD_Pinball_C"))
  (`UserWidget.AddToViewport` _returnvalue_2 0)
  (set `self.Interface` _returnvalue_2))

(event `PlayerCamera`
  (bind _returnvalue (`GameplayStatics.GetPlayerController` 0))
  ;[0.5457 1 0.4852] Ativa Câmera Player
  (bind _foundwidgets (`WidgetBlueprintLibrary.GetAllWidgetsOfClass` "/Game/Pinball/Interface/WD_Pinball.WD_Pinball_C"))
  (for _array_element _foundwidgets
    (`Widget.RemoveFromParent` _array_element)
    (`PlayerController.SetViewTargetWithBlend` _returnvalue (`GameplayStatics.GetPlayerCharacter` 0) 1.0 "VTBlend_Linear" 0.0 false)
    (`Controller.ResetIgnoreLookInput` _returnvalue)
    (`Controller.ResetIgnoreMoveInput` _returnvalue)))

(event `CriarNovaBola`
  (bind _bola (`self.Bola`))
  ;[1 0.7913 0.402] Cria Nova Bolinha
  (`/Engine/EditorBlueprintResources/StandardMacros.IsValid` _bola
    (:`Is Valid`
      (`self.K2_DestroyActor` _bola))
    (:`Is Not Valid`
      _))
  (`KismetSystemLibrary.Delay` 0.2)
  (bind _returnvalue (`|SpawnActorFromClass` "/Game/Pinball/Blueprints/BP_Ball.BP_Ball_C" (`KismetMathLibrary.MakeTransform` (`SceneComponent.K2_GetComponentLocation` (`self.BallSpawn`))) "Undefined" "OverrideRootScale" null null))
  (`/Game/Pinball/Blueprints/BP_Ball.Random Color` _returnvalue)
  (set `self.Bola` _returnvalue))

(event `/Game/Pinball/Blueprints/PinballInterface.SomaForça`
  ;[1 0.7913 0.402] Atualiza Força de Lançamento da Bolinha
  (if (and (`self.Impulse?`) (<= (`self.Impulse`) (`self.MaxImpulse`)))
    (bind _output_get (set `self.Impulse` (+ (`self.Impulse`) 10.0)))
    (`KismetSystemLibrary.PrintString` (`KismetStringLibrary.Conv_DoubleToString` _output_get))))

(event `Launch`
  ;[1 0.7913 0.402] Lança a Bolinha
  (if (`self.Impulse?`)
    (`self.EmpurrarBolinha`)))

(event `EmpurrarBolinha`
  ;[1 0.7913 0.402] Lança a Bolinha
  (`KismetSystemLibrary.Delay` 0.2)
  (`GameplayStatics.PlaySound2D` "/Game/Pinball/Assets/Sounds/Pinball_BallLaunch.Pinball_BallLaunch" 1.0 1.0 0.0 null null)
  (`PrimitiveComponent.AddImpulse` (`/Game/Pinball/Blueprints/BP_Ball.Ball` (`self.Bola`)) (* (`self.Normal Bolinha`) (`self.Impulse`)) "None" false)
  (set `self.Impulse` 0.0))

(event `self.Box1.OnComponentBeginOverlap`
  (params (OverlappedComponent :type "PrimitiveComponent Object Reference") (OtherActor :type "Actor Object Reference") (OtherComp :type "PrimitiveComponent Object Reference") (OtherBodyIndex :type Integer) (bFromSweep :type Boolean) (SweepResult :type "HitResult Structure (by ref)"))
  ;[1 0.7913 0.402] Pode Empurrar Bolinha?
  (cast `/Game/Pinball/Blueprints/BP_Ball` OtherActor)
  (set `self.Impulse?` false))

(event `self.Buraco.OnComponentHit`
  (params (HitComponent :type "PrimitiveComponent Object Reference") (OtherActor :type "Actor Object Reference") (OtherComp :type "PrimitiveComponent Object Reference") (NormalImpulse :type "Vector Structure") (Hit :type "HitResult Structure (by ref)"))
  ;[1 0.7913 0.402] Game Over
  (bind _asbp_ball (cast `/Game/Pinball/Blueprints/BP_Ball` OtherActor))
  (`self.K2_DestroyActor` _asbp_ball)
  (`self.CriarNovaBola`))

(event `self.Box1.OnComponentEndOverlap`
  (params (OverlappedComponent :type "PrimitiveComponent Object Reference") (OtherActor :type "Actor Object Reference") (OtherComp :type "PrimitiveComponent Object Reference") (OtherBodyIndex :type Integer))
  ;[1 0.7913 0.402] Pode Empurrar Bolinha?
  (cast `/Game/Pinball/Blueprints/BP_Ball` OtherActor)
  (set `self.Impulse?` true))

(event `/Game/Pinball/Blueprints/PinballInterface.FliperR P`
  ;[1 0.4125 0.855] Move Flipper Direito
  (if (`self.Tilt`)
    (bind (_direction _newtrack_0) (`Timeline|,` :!via `PlayFromStart` :!label _label)
      (:`Update`
        (`SceneComponent.K2_SetRelativeRotation` (`self.FlipperR`) (`KismetMathLibrary.RLerp` (`self.RotInicial R`) (`self.NewRot R`) _newtrack_0) false false)))))

(event `self.BumperPeq02.OnComponentHit`
  (params (HitComponent :type "PrimitiveComponent Object Reference") (OtherActor :type "Actor Object Reference") (OtherComp :type "PrimitiveComponent Object Reference") (NormalImpulse :type "Vector Structure") (Hit :type "HitResult Structure (by ref)"))
  ;[1 0.4125 0.855] Discos Repulsores
  (`/Game/Pinball/Blueprints/BumperComponent.Bump` (`self.BumperComponent`) HitComponent OtherActor (`self.StrengthBumperP`)))

(event `self.BumperPeq03.OnComponentHit`
  (params (HitComponent :type "PrimitiveComponent Object Reference") (OtherActor :type "Actor Object Reference") (OtherComp :type "PrimitiveComponent Object Reference") (NormalImpulse :type "Vector Structure") (Hit :type "HitResult Structure (by ref)"))
  ;[1 0.4125 0.855] Discos Repulsores
  (`/Game/Pinball/Blueprints/BumperComponent.Bump` (`self.BumperComponent`) HitComponent OtherActor (`self.StrengthBumperP`)))

(event `self.BumperPeq01.OnComponentHit`
  (params (HitComponent :type "PrimitiveComponent Object Reference") (OtherActor :type "Actor Object Reference") (OtherComp :type "PrimitiveComponent Object Reference") (NormalImpulse :type "Vector Structure") (Hit :type "HitResult Structure (by ref)"))
  ;[1 0.4125 0.855] Discos Repulsores
  (`/Game/Pinball/Blueprints/BumperComponent.Bump` (`self.BumperComponent`) HitComponent OtherActor (`self.StrengthBumperP`)))

(event `/Game/Pinball/Blueprints/PinballInterface.FlipperR R`
  ;[1 0.4125 0.855] Move Flipper Direito
  (if (`self.Tilt`)
    (goto _label :!via `Reverse`)))

(event `self.BumperGrande01.OnComponentHit`
  (params (HitComponent :type "PrimitiveComponent Object Reference") (OtherActor :type "Actor Object Reference") (OtherComp :type "PrimitiveComponent Object Reference") (NormalImpulse :type "Vector Structure") (Hit :type "HitResult Structure (by ref)"))
  ;[1 0.4125 0.855] Discos Repulsores
  (`/Game/Pinball/Blueprints/BumperComponent.Bump` (`self.BumperComponent`) HitComponent OtherActor (`self.StrengthBumperG`)))

(event `self.BumperGrande02.OnComponentHit`
  (params (HitComponent :type "PrimitiveComponent Object Reference") (OtherActor :type "Actor Object Reference") (OtherComp :type "PrimitiveComponent Object Reference") (NormalImpulse :type "Vector Structure") (Hit :type "HitResult Structure (by ref)"))
  ;[1 0.4125 0.855] Discos Repulsores
  (`/Game/Pinball/Blueprints/BumperComponent.Bump` (`self.BumperComponent`) HitComponent OtherActor (`self.StrengthBumperG`)))

(event `self.BumperPeq04.OnComponentHit`
  (params (HitComponent :type "PrimitiveComponent Object Reference") (OtherActor :type "Actor Object Reference") (OtherComp :type "PrimitiveComponent Object Reference") (NormalImpulse :type "Vector Structure") (Hit :type "HitResult Structure (by ref)"))
  ;[1 0.4125 0.855] Discos Repulsores
  (`/Game/Pinball/Blueprints/BumperComponent.Bump` (`self.BumperComponent`) HitComponent OtherActor (`self.StrengthBumperP`)))

(event `/Game/Pinball/Blueprints/PinballInterface.FlipperL P`
  ;[1 0.4125 0.855] Move Flipper Esquerdo
  (if (`self.Tilt`)
    (bind (_direction _newtrack_0) (`Timeline|Timeline_0` :!via `PlayFromStart` :!label _label_2)
      (:`Update`
        (bind _returnvalue (`KismetMathLibrary.RLerp` (`self.RotInicial L`) (`self.NewRot L`) _newtrack_0))
        (`SceneComponent.K2_SetRelativeRotation` (`self.FlipperL`) _returnvalue false false)
        (`SceneComponent.K2_SetRelativeRotation` (`self.FlipperPeq`) _returnvalue false false)))))

(event `/Game/Pinball/Blueprints/PinballInterface.FlipperL R`
  ;[1 0.4125 0.855] Move Flipper Esquerdo
  (if (`self.Tilt`)
    (goto _label_2 :!via `Reverse`)))

(event `Shake`
  (bind (_returnvalue_roll _returnvalue_pitch _returnvalue_yaw) (`KismetMathLibrary.BreakRotator` (`self.K2_GetActorRotation`)))
  (`self.Trapaça`)
  (bind _result (`/Engine/EditorBlueprintResources/StandardMacros.IncrementInt` (`self.Tilts`))
    (:`  `
      (bind _output_get (set `self.Tilts` _result))
      (`KismetSystemLibrary.PrintString` (`KismetStringLibrary.Conv_IntToString` _output_get))
      ;[1 0.4125 0.855] Sacudir a Máquina
      (bind (_direction _newtrack_0) (`Timeline|Shake_Pinball` :!via `PlayFromStart`)
        (:`Update`
          (`self.K2_SetActorRelativeRotation` (`KismetMathLibrary.MakeRotator` _returnvalue_roll _newtrack_0 _returnvalue_yaw)))))))

(event `Trapaça`
  ;[1 1 1] Travar Paletas
  (`KismetSystemLibrary.K2_SetTimerDelegate` (delegate `Zerar`) 2.0))

(event `Zerar`
  ;[1 1 1] Travar Paletas
  (if (and (>= (`self.Tilts`) 5) (not false))
    (set `self.Tilt` false)
    (else
      (set `self.Tilts` 0))))

(fn `UserConstructionScript`)