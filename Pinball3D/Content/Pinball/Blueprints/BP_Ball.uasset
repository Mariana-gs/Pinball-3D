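; Pinball ball Blueprint with three color states (pink, blue, white), each mapped to its own collision object channel.
; SetarCor runs on BeginPlay and applies the channel, plus a material for pink and blue only; white sets no material.
; RandomColor picks a color and reapplies it, but is not called within this Blueprint.
; On hitting a BP_Pinball, the ball writes the hit's normal impulse into that actor's NormalBolinha.
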(event `self.ReceiveBeginPlay`
  (`self.Setar Cor`))

(event `self.Ball.OnComponentHit`
  (params (HitComponent :type "PrimitiveComponent Object Reference") (OtherActor :type "Actor Object Reference") (OtherComp :type "PrimitiveComponent Object Reference") (NormalImpulse :type "Vector Structure") (Hit :type "HitResult Structure (by ref)"))
  (bind _asbp_pinball (cast `/Game/Pinball/Blueprints/BP_Pinball` OtherActor))
  (set `/Game/Pinball/Blueprints/BP_Pinball.Normal Bolinha` NormalImpulse _asbp_pinball))

(fn `Random Color`
  (switch `int` (`KismetMathLibrary.RandomInteger` 3)
    (:`0`
      (set `self.Color` "NewEnumerator0"))
    (:`1`
      (set `self.Color` "NewEnumerator1"))
    (:`2`
      (set `self.Color` "NewEnumerator2")))
  (`self.Setar Cor`))

(fn `Setar Cor`
  (switch `/Game/Pinball/Blueprints/Colors` (`self.Color`)
    (:`NewEnumerator0`
      (`PrimitiveComponent.SetMaterial` (`self.Ball`) 0 "/Game/Pinball/Material/M_Pink.M_Pink")
      (`PrimitiveComponent.SetCollisionObjectType` (`self.Ball`) "ECC_GameTraceChannel2"))
    (:`NewEnumerator1`
      (`PrimitiveComponent.SetMaterial` (`self.Ball`) 0 "/Game/Pinball/Material/MI_Blue.MI_Blue")
      (`PrimitiveComponent.SetCollisionObjectType` (`self.Ball`) "ECC_GameTraceChannel3"))
    (:`NewEnumerator2`
      (`PrimitiveComponent.SetCollisionObjectType` (`self.Ball`) "ECC_GameTraceChannel1"))))

(fn `UserConstructionScript`)